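; Character stat Blueprint that tracks health and stamina, starting both at their maximums.
; SetHP clamps health and fires the OnHP dispatcher, plus OnDead at zero; MakeDamage routes through it and prints the damage source.
; Each Tick, UpdateBio drains stamina while sprinting or regenerates it otherwise, then allows sprinting only while stamina is above a fixed threshold.
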(event EventBeginPlay
  (CallFunction|SetHP (Variables|Default|GetMaxHP))
  (Variables|Default|SetStamina (Variables|Default|GetMaxStamina)))

(event EventTick
  (params (DeltaSeconds :type Float%20%28single-precision%29))
  (CallFunction|UpdateBio DeltaSeconds))

(fn SetHP
  (params (Value :type Float%20%28single-precision%29))
  (Variables|Default|SetHP (Math|Float|Clamp(Float) Value 0.0 (Variables|Default|GetMaxHP)))
  (Default|CallOnHP)
  (if (== (Variables|Default|GetHP) 0.0)
    (Default|CallOnDead)))

(fn MakeDamage
  (params (Damage :type Float%20%28single-precision%29) (WhoDamage :type Actor%20Object%20Reference))
  (CallFunction|SetHP (- (Variables|Default|GetHP) Damage))
  (Development|PrintString (Utilities|String|Append "Damage from: " (Utilities|GetDisplayName WhoDamage)) true true "(R=0.205739,G=0.267334,B=0.214003,A=0.716000)" 1.0))

(fn UpdateBio
  (params (Delta :type Float%20%28single-precision%29))
  (Utilities|FlowControl|Sequence
    (:then_0
      ;[1 1 1] Обновление выносливости
      (if (Variables|Default|GetOnSprint)
        (Variables|Default|SetStamina (Math|Float|Clamp(Float) (- (Variables|Default|GetStamina) (* Delta (Variables|Default|GetStaminaSubstract))) 0.0 (Variables|Default|GetMaxStamina)))
        (else
          (Variables|Default|SetStamina (Math|Float|Clamp(Float) (+ (* Delta (Variables|Default|GetStaminaRegen)) (Variables|Default|GetStamina)) 0.0 (Variables|Default|GetMaxStamina))))))
    (:then_1
      (Variables|Default|SetCanUseSprint (> (Variables|Default|GetStamina) 2e+01)))))