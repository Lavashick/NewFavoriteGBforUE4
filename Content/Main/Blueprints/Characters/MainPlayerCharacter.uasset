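; Player character Blueprint with mouse-wheel camera zoom and weapon pickup.
; CameraUp and CameraDown inputs change the spring arm length by a set step within clamped limits.
; HasWeapon stores a candidate weapon; Activate calls TakeWeapon, which makes it active, snaps it to a Scene component and disables its mesh physics.
; ActivateObject gates this on the current ActiveWeapon being valid, rather than the candidate.
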(event EventBeginPlay)

(event Collision|EventActorBeginOverlap
  (params (OtherActor :type Actor%20Object%20Reference)))

(event EventTick
  (params (DeltaSeconds :type Float%20%28single-precision%29)))

(event Input|ActionEvents|InputActionCameraUp
  (params (Key :type Key%20Structure :default "None"))
  ;[1 1 1] Приближение/отдаление колесика мыши
  (:Pressed
    (Variables|/Script/Engine.SpringArmComponent|SetTargetArmLength (Variables|Default|GetSpringArm) (Math|Float|Clamp(Float) (+ (Variables|/Script/Engine.SpringArmComponent|GetTargetArmLength (Variables|Default|GetSpringArm)) (Variables|Default|GetCameraDif)) 1.5e+02 7e+02))))

(event Input|ActionEvents|InputActionCameraDown
  (params (Key :type Key%20Structure :default "None"))
  ;[1 1 1] Приближение/отдаление колесика мыши
  (:Pressed
    (Variables|/Script/Engine.SpringArmComponent|SetTargetArmLength (Variables|Default|GetSpringArm) (Math|Float|Clamp(Float) (- (Variables|/Script/Engine.SpringArmComponent|GetTargetArmLength (Variables|Default|GetSpringArm)) (Variables|Default|GetCameraDif)) 1.5e+02 7e+02))))

(event Input|ActionEvents|InputActionActivate
  (params (Key :type Key%20Structure :default "None"))
  (:Pressed
    (CallFunction|ActivateObject)))

(fn ConstructionScript)

(fn HasWeapon
  (params (Weapon :type Base%20Weapon%20Object%20Reference))
  (Variables|Default|SetActivatingWeapon Weapon))

(fn ActivateObject
  (if (Utilities|IsValid (Variables|Default|GetActiveWeapon))
    (CallFunction|TakeWeapon)))

(fn TakeWeapon
  (bind _output_get (Variables|Default|SetActiveWeapon (Variables|Default|GetActivatingWeapon)))
  (Transformation|AttachComponentToComponent _output_get (Variables|Default|GetScene) "None" "SnapToTarget" "SnapToTarget" "KeepRelative" true)
  (Physics|SetSimulatePhysics (Variables|/Game/Main/BaseObjects/Interract/BaseWeapon.BaseWeapon_C|GetSkeletalMesh (Variables|Default|GetActiveWeapon)) false))