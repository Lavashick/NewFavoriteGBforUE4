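; Base damage zone actor that deals continuous damage to actors inside its Box volume.
; Box begin and end overlap events add actors to and remove them from the DamageActor array, with no filtering by type.
; Every Tick sends a DoDamage interface message to each tracked actor with Damage scaled by DeltaSeconds, so Damage acts as a per-second rate.
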(event OnComponentBeginOverlap(Box)
  (params (OverlappedComponent :type Primitive%20Component%20Object%20Reference) (OtherActor :type Actor%20Object%20Reference) (OtherComp :type Primitive%20Component%20Object%20Reference) (OtherBodyIndex :type Integer) (bFromSweep :type Boolean) (SweepResult :type Hit%20Result%20Structure%20%28by%20ref%29))
  ;[1 1 1] Вход/выход из зоны
  (Utilities|Array|AddUnique (Variables|Default|GetDamageActor) OtherActor))

(event OnComponentEndOverlap(Box)
  (params (OverlappedComponent :type Primitive%20Component%20Object%20Reference) (OtherActor :type Actor%20Object%20Reference) (OtherComp :type Primitive%20Component%20Object%20Reference) (OtherBodyIndex :type Integer))
  ;[1 1 1] Вход/выход из зоны
  (Utilities|Array|RemoveItem (Variables|Default|GetDamageActor) OtherActor))

(event EventBeginPlay)

(event Collision|EventActorBeginOverlap
  (params (OtherActor :type Actor%20Object%20Reference)))

(event EventTick
  (params (DeltaSeconds :type Float%20%28single-precision%29))
  ;[1 1 1] Получение дамага персонажем
  (if (> (Utilities|Array|Length (Variables|Default|GetDamageActor)) 0)
    (for _array_element (Variables|Default|GetDamageActor)
      (Class|Damage|DoDamage(Message) _array_element (* (Variables|Default|GetDamage) DeltaSeconds)))))

(fn ConstructionScript)